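; Mordhau mod actor for "Dogmod" combat: no chambers, morphs or ripostes, slower unfeintable stabs, restricted feints and no health regen.
; The authority keeps one instance and starts a one-second timer that re-edits every character's motions and weapon attacks.
; Tick adjusts the local player's current motion windows and stamina-based movement, feeding a feint countdown widget.
; Outside PIE, admins toggle the saved Enabled setting with ".contingent" in chat.
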(event `InputAction|Parry`
  (params (Key :type "Key Structure"))
  (:`Pressed`
    (bind _asstab_motion (cast `StabMotion` (`AdvancedCharacter.GetMotion` (`self.MyChar`)) :!label _label))
    (set `AttackMotion.FeintWindow` 0.0 _asstab_motion)
    (`KismetSystemLibrary.PrintString` "stab to parry")))

(event `InputAction|Feint Or Parry`
  (params (Key :type "Key Structure"))
  (:`Pressed`
    (goto _label)))

(event `self.ReceiveBeginPlay`
  (bind (_isvalid _returnvalue) (`MordhauUtilityLibrary.GetCustomConfigVar_Bool` "ContingentLite" "Enabled"))
  (`KismetSystemLibrary.Delay` 5.0)
  (`/Engine/EditorBlueprintResources/ActorMacros.Switch Has Authority`
    (:`Authority`
      (bind _outactors (`GameplayStatics.GetAllActorsOfClass` "BP_Contingent_C"))
      (for (_array_element _array_index) _outactors
        (if (> _array_index 0)
          (`self.K2_DestroyActor` _array_element)))
      (`KismetSystemLibrary.K2_SetTimerDelegate` (delegate `SRV Combat Change`) 1.0 true)
      (if (not (`MordhauUtilityLibrary.IsPlayInEditor`))
        (bind _asmordhau_game_mode (cast `MordhauGameMode` (`GameplayStatics.GetGameMode`)))
        (add `MordhauGameMode.OnMessageBroadcasted` _asmordhau_game_mode (delegate `CustomEvent_0`))
        (if _isvalid
          (set `self.Enabled?` _returnvalue)
          (else
            (`MordhauUtilityLibrary.SetCustomConfigVar_Bool` "ContingentLite" "Enabled" true)
            (set `self.Enabled?` true)))
        (`MordhauGameMode.Broadcast` _asmordhau_game_mode null (`KismetStringLibrary.Concat_StrStr` "Dogmod combat is " (select `bool` (`self.Enabled?`) :`false` "disabled." :`true` "enabled.")) "ServerSay")
        (if (`self.Enabled?`)
          (`MordhauGameMode.Broadcast` _asmordhau_game_mode null (`KismetTextLibrary.Conv_TextToString` (`|FormatText` "- No Chamber \n- No Morph \n- No Riposte \n- Stabs have {swindup} windup and can't be feinted \n- No combo on miss \n- Strike feint window {sfeint}%" (`self.StabWindup`) (* (- 1.0 (`self.FeintWindowStrikes`)) 100.0))) "ServerSay"))))))

(event `CustomEvent_0`
  (params (Sender :type "Actor Object Reference") (Msg :type String) (Type :type Name))
  (bind _returnvalue (not (`.ReturnValue` (`MordhauUtilityLibrary.GetCustomConfigVar_Bool` "ContingentLite" "Enabled"))))
  (bind _asmordhau_player_controller (cast `MordhauPlayerController` Sender))
  (if (`MordhauPlayerController.IsAdmin` _asmordhau_player_controller)
    (if (`KismetStringLibrary.Contains` Msg ".contingent")
      (bind _output_get (set `self.Enabled?` _returnvalue))
      (`MordhauUtilityLibrary.SetCustomConfigVar_Bool` "ContingentLite" "Enabled" _returnvalue)
      (`MordhauGameMode.Broadcast` (cast `MordhauGameMode` (`GameplayStatics.GetGameMode`) :!pure true) null (`KismetStringLibrary.Concat_StrStr` "Dogmod combat " (select `bool` _output_get :`false` "disabled. (May need to restart map!)" :`true` "enabled. (May need to restart map!)")) "ServerSay"))))

(event `SRV Combat Change`
  (`self.ModifyCombat`))

(event `ModifyCombat`
  (if (`self.Enabled?`)
    (`self.EditAllChars`)
    (`KismetSystemLibrary.K2_ClearAndInvalidateTimerHandle` (`self.MotionEditingTimer`))
    (`self.Disable Health Regen`)
    (`/Engine/EditorBlueprintResources/StandardMacros.DoOnce` false
      (:`Completed`
        (bind _asbp_mordhau_hud (cast `/Game/Mordhau/Blueprints/BP_MordhauHUD` (`PlayerController.GetHUD` (`GameplayStatics.GetPlayerController` 0))))
        (`/Game/Mordhau/Blueprints/BP_MordhauHUD.ShowAnnouncement` _asbp_mordhau_hud "Dogmod enabled!" "- No Chamber \n- No Morph \n- No Riposte \n- Feints punishable with all stabs" 8.0 "NewEnumerator1")
        (bind _returnvalue (`|CreateWidget` "/ContingentLite/BP_Cooldown.BP_Cooldown_C"))
        (`UserWidget.AddToViewport` _returnvalue -10)
        (set `self.CooldownRef` _returnvalue)))))

(event `self.ReceiveTick`
  (params (DeltaSeconds :type "Float (single-precision)"))
  (if (`self.Enabled?`)
    (`self.EditMyMotions`)))

(event `Disable Health Regen`
  (bind _returnvalue (`GameplayStatics.GetGameState`))
  (bind _asbp_deathmatch_game_state (cast `/Game/Mordhau/Blueprints/GameModes/BP_DeathmatchGameState` _returnvalue)
    (:`then`
      (set `MordhauGameState.WarmupEnd` 0.0 _asbp_deathmatch_game_state)
      (set `MordhauGameState.bAllowHealthRegen` false _asbp_deathmatch_game_state))
    (:`CastFailed`
      (bind _asbp_skirmish_game_state (cast `/Game/Mordhau/Blueprints/GameModes/Skirmish/BP_SkirmishGameState` _returnvalue))
      (set `MordhauGameState.bAllowHealthRegen` false _asbp_skirmish_game_state))))

(event `SRV Modify Chamber Values`
  (if (`self.Enabled?`)
    (for _array_element (`self.AllChars`)
      (bind _returnvalue (`AdvancedCharacter.GetMotion` _array_element))
      (bind _asstab_motion (cast `StabMotion` _returnvalue)
        (:`then`
          (set `AttackMotion.ClashAngle` 180.0 _asstab_motion)
          (set `AttackMotion.EarlyReleaseIsClashableAfter` 0.0 _asstab_motion))
        (:`CastFailed`
          (bind _asstrike_motion (cast `StrikeMotion` _returnvalue))
          (set `AttackMotion.ClashAngle` 0.0 _asstrike_motion)
          (set `AttackMotion.EarlyReleaseIsClashableAfter` 1.0 _asstrike_motion))))))

(fn `Cap Array`
  (params (`In Array` :type "Array of Float (double-precision)") (Max :type "Float (double-precision)"))
  (returns (`Out Array` :type "Array of Float (double-precision)"))
  (locals (NewLocalVar_0 :type "Array of Float (double-precision)"))
  (bind _output_get (set `local.NewLocalVar_0` `In Array`))
  (for (_array_element _array_index) _output_get
    (if (> _array_element Max)
      (`KismetArrayLibrary.Array_Set` (`local.NewLocalVar_0`) _array_index Max)))
  (return (`local.NewLocalVar_0`)))

(fn `Disable Riposte`
  (params (`Attack Motion` :type "AttackMotion Object Reference"))
  (set `AttackMotion.RiposteWindupModifier` 1.0 `Attack Motion`)
  (set `AttackMotion.RiposteBlendIn` (`AttackMotion.NormalBlendIn` `Attack Motion`) `Attack Motion`)
  (set `AttackMotion.RiposteReleaseCurve` (`AttackMotion.ReleaseCurve` `Attack Motion`) `Attack Motion`)
  (set `AttackMotion.RiposteAnimation` (`AttackMotion.Animation` `Attack Motion`) `Attack Motion`)
  (set `AttackMotion.bIsRiposteFeintable` true `Attack Motion`)
  (return))

(fn `Display Cooldown`
  (params (Duration :type "Float (double-precision)"))
  (`/Game/Mordhau/UI/Shared/BP_CircleTimer.Start Countdown` (`/ContingentLite/BP_Cooldown.BP_CircleTimer` (`self.CooldownRef`)) Duration))

(fn `EditAllChars`
  (locals (IsDeathmatch :type Boolean))
  (set `local.IsDeathmatch` (`.bSuccess` (cast `/Game/Mordhau/Blueprints/GameModes/BP_DeathmatchGameState` (`GameplayStatics.GetGameState`) :!pure true)))
  (bind _outactors (`GameplayStatics.GetAllActorsOfClass` "/Game/Mordhau/Blueprints/Characters/BP_MordhauCharacter.BP_MordhauCharacter_C"))
  (bind _output_get (set `self.AllChars` _outactors))
  (for _array_element _output_get
    (`|ExecutionSequence`
      (:`then_0`
        (`self.EditChar` _array_element))
      (:`then_1`
        (if (`local.IsDeathmatch`)
          (set `MordhauCharacter.HealthOnKill` 100 _array_element)
          (set `MordhauCharacter.StaminaOnKill` 100 _array_element)))
      (:`then_2`
        (cast `/Game/Mordhau/Blueprints/Equipment/Weapons/BP_MordhauWeapon` (`MordhauCharacter.RightHandEquipment` _array_element)))
      (:`then_3`
        (`/Engine/EditorBlueprintResources/StandardMacros.Can Execute Cosmetic Events`
          (:`True`
            (if (== (`Controller.PlayerState` (`GameplayStatics.GetPlayerController` 0)) (`Pawn.PlayerState` _array_element))
              (set `self.MyChar` _array_element))))))))

(fn `EditChar`
  (params (Char :type "MordhauCharacter Object Reference (by ref)"))
  (bind _motions (`MordhauCharacter.Motions` Char))
  (bind _stabwindup (`self.StabWindup`))
  (bind _stabrelease (`self.StabRelease`))
  (bind _no_release_flinch_on_stabs (`self.No Release Flinch on Stabs`))
  (bind _feint_cost (`self.Feint Cost`))
  ;[1 1 1] removed knockback
  (set `MordhauCharacter.KnockbackParry` 0.0 Char)
  (set `MordhauCharacter.KnockbackClash` 0.0 Char)
  (set `AdvancedCharacter.FootstepVolumeModifierEnemy` 1.5 Char)
  (`KismetArrayLibrary.Array_Set` _motions 2 "/ContingentLite/BP_ParryMotion_CTG.BP_ParryMotion_CTG_C")
  (`KismetArrayLibrary.Array_Set` _motions 5 "/ContingentLite/BP_FeintedMotion_CTG.BP_FeintedMotion_CTG_C")
  (`KismetArrayLibrary.Array_Set` _motions 6 "/ContingentLite/BP_BlockedMotion_CTG.BP_BlockedMotion_CTG_C")
  (set `MordhauCharacter.bCannotChamber` true Char)
  (bind _asmordhau_weapon (cast `MordhauWeapon` (`MordhauCharacter.RightHandEquipment` Char)))
  (bind _structout (setmembers `AttackInfo` :`StructRef` (`MordhauWeapon.StrikeAttack` _asmordhau_weapon) :`bCanMissCombo` false :`FeintCost` _feint_cost))
  (set `MordhauWeapon.StrikeAttack` _structout _asmordhau_weapon)
  (bind _structout_2 (setmembers `AttackInfo` :`StructRef` (`MordhauWeapon.SecondStrikeAttack` _asmordhau_weapon) :`bCanMissCombo` false :`FeintCost` _feint_cost))
  (set `MordhauWeapon.SecondStrikeAttack` _structout_2 _asmordhau_weapon)
  (bind _structout_3 (setmembers `AttackInfo` :`StructRef` (`MordhauWeapon.StabAttack` _asmordhau_weapon) :`bCanMissCombo` false :`bNoReleaseFlinch` _no_release_flinch_on_stabs :`Windup` _stabwindup :`ComboWindupIncrease` 0.4 :`Release` _stabrelease))
  (set `MordhauWeapon.StabAttack` _structout_3 _asmordhau_weapon)
  (bind _structout_4 (setmembers `AttackInfo` :`StructRef` (`MordhauWeapon.SecondStabAttack` _asmordhau_weapon) :`bCanMissCombo` false :`bNoReleaseFlinch` _no_release_flinch_on_stabs :`Windup` _stabwindup :`ComboWindupIncrease` 0.4 :`Release` _stabrelease))
  (set `MordhauWeapon.SecondStabAttack` _structout_4 _asmordhau_weapon))

(fn `EditMyMotions`
  (locals (IsPanting :type Boolean :default false))
  (bind _mychar (`self.MyChar`))
  (bind _returnvalue (`AdvancedCharacter.GetMotion` (`self.MyChar`)))
  (bind _returnvalue_2 (`StatComponent.GetStatValue` (`AdvancedCharacter.StaminaStatComponent` _mychar)))
  (bind _returnvalue_3 (<= _returnvalue_2 15))
  (`|ExecutionSequence`
    (:`then_0`
      (if (not (`|EnumEquality` (`MordhauCharacter.GetMovementRestriction` _mychar) "NoMovement"))
        (set `local.IsPanting` _returnvalue_3)
        (if _returnvalue_3
          (set `MordhauMotion.MovementRestriction` (select `bool` (== _returnvalue_2 0) :`false` "PartialSprint" :`true` "Walk" :!type "EMovementRestriction Enum") _returnvalue)
          (else
            (set `MordhauMotion.MovementRestriction` "None" _returnvalue)))))
    (:`then_1`
      (bind _asstab_motion (cast `StabMotion` _returnvalue)
        (:`then`
          (set `AttackMotion.MorphWindow` 0.0 _asstab_motion)
          (set `AttackMotion.FeintWindow` 1.0 _asstab_motion))
        (:`CastFailed`
          (bind _asstrike_motion (cast `StrikeMotion` _returnvalue)
            (:`then`
              (set `AttackMotion.MorphWindow` 0.0 _asstrike_motion)
              (if (> (`AttackMotion.AngleTarget` _asstrike_motion) 0.01)
                (bind _output_get (set `AttackMotion.FeintWindow` 0.25 _asstrike_motion))
                (bind _windupend (`AttackMotion.WindupEnd` _asstrike_motion))
                (`self.Display Cooldown` (- (- _windupend _output_get) (`GameplayStatics.GetTimeSeconds`)))
                (elif (`MordhauMotion.bIsFlinchable` _returnvalue)
                  (bind _output_get_2 (set `AttackMotion.FeintWindow` (`self.FeintWindowStrikes`) _asstrike_motion))
                  (`self.Display Cooldown` (- (- _windupend _output_get_2) (`GameplayStatics.GetTimeSeconds`)))
                  (else
                    (`self.Hide Cooldown`)))))
            (:`CastFailed`
              (bind _asparry_motion (cast `ParryMotion` _returnvalue)
                (:`then`
                  (set `ParryMotion.QueuedMoveTime` -10000.0 _asparry_motion)
                  (`self.Hide Cooldown`)
                  (set `ParryMotion.RiposteWindowBase` -100.0 _asparry_motion)
                  (set `ParryMotion.RiposteWindowStart` -100.0 _asparry_motion)
                  (set `ParryMotion.NonHeldParryExtensionAndRiposteWindowExtra` 0.0 _asparry_motion))
                (:`CastFailed`
                  (`self.Hide Cooldown`))))))))))

(fn `Hide Cooldown`
  (`/Game/Mordhau/UI/Shared/BP_CircleTimer.Start Countdown` (`/ContingentLite/BP_Cooldown.BP_CircleTimer` (`self.CooldownRef`)) 0.0))

(fn `UserConstructionScript`)